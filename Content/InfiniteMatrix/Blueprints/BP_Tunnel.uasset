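; Tunnel segment for an endless flight game, holding a rotating holed wall, a rotating health pickup and a shootable enemy.
; Its trigger has TunnelSpawner spawn the next segment, destroys this one, and awards a point and extra speed unless the wall was hit.
; Overlaps adjust player health, trigger death and restart, consume projectiles, or score enemy kills.
; Randomize functions vary meshes, wall rotation and item placement, but are not called here.
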(event `self.ReceiveTick`
  (params (DeltaSeconds :type "Float (single-precision)"))
  (bind _returnvalue (* DeltaSeconds (`self.RotateSpeed`)))
  (`SceneComponent.K2_AddLocalRotation` (`self.WallMesh`) (`KismetMathLibrary.MakeRotator` (* DeltaSeconds (`self.RotateSpeed`))) false false)
  (`SceneComponent.K2_AddLocalRotation` (`self.HealthPack`) (`KismetMathLibrary.MakeRotator` _returnvalue 0.0 _returnvalue) false false))

(event `self.TriggerZone.OnComponentBeginOverlap`
  (params (OverlappedComponent :type "PrimitiveComponent Object Reference") (OtherActor :type "Actor Object Reference") (OtherComp :type "PrimitiveComponent Object Reference") (OtherBodyIndex :type Integer) (bFromSweep :type Boolean) (SweepResult :type "HitResult Structure (by ref)"))
  (cast `/Game/InfiniteMatrix/Blueprints/BP_Player` OtherActor)
  (`/Game/InfiniteMatrix/Blueprints/BP_TunnelSpawner.SpawnTunnelAtSpawnPoint` (`self.TunnelSpawner`))
  (`self.K2_DestroyActor`)
  (if (`self.Collide_flag`)
    (set `self.Collide_flag` false)
    (else
      (bind _asbp_player (cast `/Game/InfiniteMatrix/Blueprints/BP_Player` OtherActor))
      (set `/Game/InfiniteMatrix/Blueprints/BP_Player.Points` (+ (`/Game/InfiniteMatrix/Blueprints/BP_Player.Points` _asbp_player) 1) _asbp_player)
      (set `self.Collide_flag` false)
      (set `/Game/InfiniteMatrix/Blueprints/BP_Player.FowardSpeed` (+ (`/Game/InfiniteMatrix/Blueprints/BP_Player.FowardSpeed` _asbp_player) 75.0) _asbp_player))))

(event `self.WallMesh.OnComponentBeginOverlap`
  (params (OverlappedComponent :type "PrimitiveComponent Object Reference") (OtherActor :type "Actor Object Reference") (OtherComp :type "PrimitiveComponent Object Reference") (OtherBodyIndex :type Integer) (bFromSweep :type Boolean) (SweepResult :type "HitResult Structure (by ref)"))
  (bind _asbp_projectile (cast `/Game/InfiniteMatrix/Blueprints/BP_Projectile` OtherActor)
    (:`then`
      (`self.K2_DestroyActor` _asbp_projectile))
    (:`CastFailed`
      (set `self.Collide_flag` true)
      (bind _asbp_player (cast `/Game/InfiniteMatrix/Blueprints/BP_Player` OtherActor))
      (bind _output_get (set `/Game/InfiniteMatrix/Blueprints/BP_Player.Health` (- (`/Game/InfiniteMatrix/Blueprints/BP_Player.Health` _asbp_player) 1.0) _asbp_player))
      (if (<= _output_get 0.0)
        (set `/Game/InfiniteMatrix/Blueprints/BP_Player.IsDead` true _asbp_player)
        (`/Game/InfiniteMatrix/Blueprints/BP_Player. DisplayRestart` _asbp_player)))))

(event `self.HealthPack.OnComponentBeginOverlap`
  (params (OverlappedComponent :type "PrimitiveComponent Object Reference") (OtherActor :type "Actor Object Reference") (OtherComp :type "PrimitiveComponent Object Reference") (OtherBodyIndex :type Integer) (bFromSweep :type Boolean) (SweepResult :type "HitResult Structure (by ref)"))
  (bind _asbp_projectile (cast `/Game/InfiniteMatrix/Blueprints/BP_Projectile` OtherActor)
    (:`then`
      (`self.K2_DestroyActor` _asbp_projectile))
    (:`CastFailed`
      (bind _asbp_player (cast `/Game/InfiniteMatrix/Blueprints/BP_Player` OtherActor))
      (if (< (`/Game/InfiniteMatrix/Blueprints/BP_Player.Health` _asbp_player) 3.0)
        (set `/Game/InfiniteMatrix/Blueprints/BP_Player.Health` (+ (`/Game/InfiniteMatrix/Blueprints/BP_Player.Health` _asbp_player) 0.5) _asbp_player)))))

(event `self.Enemy.OnComponentBeginOverlap`
  (params (OverlappedComponent :type "PrimitiveComponent Object Reference") (OtherActor :type "Actor Object Reference") (OtherComp :type "PrimitiveComponent Object Reference") (OtherBodyIndex :type Integer) (bFromSweep :type Boolean) (SweepResult :type "HitResult Structure (by ref)"))
  (bind _asbp_player (cast `/Game/InfiniteMatrix/Blueprints/BP_Player` OtherActor)
    (:`then`
      (`ActorComponent.K2_DestroyComponent` (`self.Enemy`))
      (set `/Game/InfiniteMatrix/Blueprints/BP_Player.Health` (- (`/Game/InfiniteMatrix/Blueprints/BP_Player.Health` _asbp_player) 0.75) _asbp_player)
      (if (<= (`/Game/InfiniteMatrix/Blueprints/BP_Player.Health` _asbp_player) 0.0)
        (set `/Game/InfiniteMatrix/Blueprints/BP_Player.IsDead` true _asbp_player)
        (`/Game/InfiniteMatrix/Blueprints/BP_Player. DisplayRestart` _asbp_player)))
    (:`CastFailed`
      (bind _asbp_projectile (cast `/Game/InfiniteMatrix/Blueprints/BP_Projectile` OtherActor))
      (`ActorComponent.K2_DestroyComponent` (`self.Enemy`))
      (`self.K2_DestroyActor` _asbp_projectile)
      (bind _asbp_player_2 (cast `/Game/InfiniteMatrix/Blueprints/BP_Player` (`GameplayStatics.GetPlayerPawn` 0)))
      (set `/Game/InfiniteMatrix/Blueprints/BP_Player.Points` (+ (`/Game/InfiniteMatrix/Blueprints/BP_Player.Points` _asbp_player_2) 3) _asbp_player_2))))

(fn `RandomizeEnemy`
  (`StaticMeshComponent.SetStaticMesh` (`self.Enemy`) (select `int` (`KismetMathLibrary.RandomIntegerInRange` 0) :`0` "/Game/Megascans/3D_Assets/Animal_Skull_wk5hfcl/S_Animal_Skull_wk5hfcl_lod3_Var1.S_Animal_Skull_wk5hfcl_lod3_Var1" :`1` null :`2` null :`3` null :!type "StaticMesh Object Reference"))
  (`SceneComponent.K2_SetRelativeLocation` (`self.Enemy`) (`KismetMathLibrary.MakeVector` 1000.0 (`KismetMathLibrary.RandomFloatInRange` -300.0 300.0) (`KismetMathLibrary.RandomFloatInRange` -300.0 300.0)) false false))

(fn `RandomizeHealthPack`
  (`StaticMeshComponent.SetStaticMesh` (`self.HealthPack`) (select `int` (`KismetMathLibrary.RandomIntegerInRange` 0) :`0` "/Game/Megascans/3D_Assets/Banana_vfendgyiw/S_Banana_vfendgyiw_lod3_Var1.S_Banana_vfendgyiw_lod3_Var1" :`1` null :`2` null :`3` null :!type "StaticMesh Object Reference"))
  (`SceneComponent.K2_AddLocalRotation` (`self.HealthPack`) (`KismetMathLibrary.MakeRotator` (`KismetMathLibrary.RandomFloatInRange` 0.0 360.0)) false false)
  (`SceneComponent.K2_SetRelativeLocation` (`self.HealthPack`) (`KismetMathLibrary.MakeVector` 1500.0 (`KismetMathLibrary.RandomFloatInRange` -300.0 300.0) (`KismetMathLibrary.RandomFloatInRange` -300.0 300.0)) false false))

(fn `RandomizeWall`
  (`StaticMeshComponent.SetStaticMesh` (`self.WallMesh`) (select `int` (`KismetMathLibrary.RandomIntegerInRange` 0 3) :`0` "/Game/InfiniteMatrix/Meshes/SM_Hole_01.SM_Hole_01" :`1` "/Game/InfiniteMatrix/Meshes/SM_Hole_02.SM_Hole_02" :`2` "/Game/InfiniteMatrix/Meshes/SM_Hole_03.SM_Hole_03" :`3` "/Game/InfiniteMatrix/Meshes/SM_Hole_04.SM_Hole_04" :!type "StaticMesh Object Reference"))
  (`SceneComponent.K2_AddLocalRotation` (`self.WallMesh`) (`KismetMathLibrary.MakeRotator` (`KismetMathLibrary.RandomFloatInRange` 0.0 360.0)) false false))

(fn `UserConstructionScript`)